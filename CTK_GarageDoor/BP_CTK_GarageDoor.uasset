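; A usable, destructible garage door that slides vertically between open and closed, starting in the state set by DoorOpen.
; Use toggles it through Server-to-Client event pairs that play Timelines with Wwise sound, with CanOpen blocking input mid-move.
; A box overlap by non-player-controlled actors also triggers opening, delayed if the door is busy.
; Radial damage drains Health, and a polling timer hides the door and disables its collision once depleted.
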(event OnComponentBeginOverlap(Box)
  (params (OverlappedComponent :type Primitive%20Component%20Object%20Reference) (OtherActor :type Actor%20Object%20Reference) (OtherComp :type Primitive%20Component%20Object%20Reference) (OtherBodyIndex :type Integer) (bFromSweep :type Boolean) (SweepResult :type Hit%20Result%20Structure%20%28by%20ref%29))
  (if (not (Class|Controller|IsPlayerController (Game|GetInstigatorController OtherActor)))
    (if (Variables|Default|GetCanOpen?)
      _
      (else
        (Utilities|FlowControl|Delay 8.0)))
    (CallFunction|OpenServer)))

(event Custom|Open%20Server
  (CallFunction|OpenClient))

(event Custom|Close%20Client
  (Variables|Default|SetCanOpen? false)
  (bind _newtrack_0 (Timeline|Timeline_3 PlayFromStart)
    (:Update
      (Transformation|SetRelativeLocation (Variables|Default|GetGarageDoor) (Math|Vector|MakeVector 3.3 -18.5 _newtrack_0) false false)
      (Class|AkGameObject|PostAkEvent (Variables|Default|GetSound%28opening%29) "/Game/Audio/wwise/Sandstorm/Physics/Dynamic_Props/Breakable/Play_Metal_Small_Breakable_Prop.Play_Metal_Small_Breakable_Prop"))
    (:Finished
      (Utilities|FlowControl|Delay 0.5)
      (Variables|Default|SetDoorOpen false)
      (Variables|Default|SetCanOpen? true))))

(event Custom|Open%20Client
  (Variables|Default|SetCanOpen? false)
  (bind _newtrack_0 (Timeline|Timeline_0 PlayFromStart)
    (:Update
      (Transformation|SetRelativeLocation (Variables|Default|GetGarageDoor) (Math|Vector|MakeVector 3.3 -18.5 _newtrack_0) false false)
      (Class|AkGameObject|PostAkEvent (Variables|Default|GetSound%28opening%29) "/Game/Audio/wwise/Sandstorm/Physics/Dynamic_Props/Breakable/Play_Metal_Small_Breakable_Prop.Play_Metal_Small_Breakable_Prop"))
    (:Finished
      (Utilities|FlowControl|Delay 0.5)
      (Variables|Default|SetDoorOpen true)
      (Variables|Default|SetCanOpen? true))))

(event Custom|Switch
  (Utilities|FlowControl|RetriggerableDelay 0.5)
  (if (Variables|Default|GetCanOpen?)
    (if (Variables|Default|GetDoorOpen)
      (CallFunction|CloseServer)
      (else
        (CallFunction|OpenServer)))))

(event Custom|Close%20Server
  (CallFunction|CloseClient))

(event Custom|Timer
  (Utilities|FlowControl|Delay 0.5)
  (if (<= (Variables|Default|GetHealth) 1)
    (Utilities|FlowControl|DoOnce false
      (:Completed
        (CallFunction|DestroyClient)))
    (else
      (CallFunction|Timer))))

(event Custom|DestroyClient
  (bind _garagedoor (Variables|Default|GetGarageDoor))
  ;[1 1 1] Need Server?
  (Rendering|SetVisibility _garagedoor false false)
  (Collision|SetCollisionEnabled _garagedoor "NoCollision"))

(event EventBeginPlay
  (CallFunction|Timer)
  (Class|AkComponent|SetOutputBusVolume (Variables|Default|GetSound%28opening%29) 0.075)
  (Class|AkComponent|SetOutputBusVolume (Variables|Default|GetSound%28destroy%29) 0.5)
  (Class|AkGameObject|PostAkEvent (Variables|Default|GetSound%28destroy%29) "/Game/Audio/wwise/Sandstorm/Vehicles/Land/SharedAssets/Play_Vehicle_Hood_Destroyed.Play_Vehicle_Hood_Destroyed"))

(event Game|Damage|EventRadialDamage
  (params (DamageReceived :type Float%20%28single-precision%29) (DamageType :type Damage%20Type%20Object%20Reference) (Origin :type Vector :default "0, 0, 0") (HitInfo :type Hit%20Result%20Structure%20%28by%20ref%29) (InstigatedBy :type Controller%20Object%20Reference) (DamageCauser :type Actor%20Object%20Reference))
  (Variables|Default|SetHealth (- (Variables|Default|GetHealth) (Math|Float|Truncate DamageReceived)))
  (Class|AkGameObject|PostAkEvent (Variables|Default|GetSound%28destroy%29) "/Game/Audio/wwise/Sandstorm/Vehicles/Land/SharedAssets/Play_Vehicle_Hood_Destroyed.Play_Vehicle_Hood_Destroyed")
  (Components|Activation|Activate (Variables|Default|GetParticleSystem) false))

(fn ConstructionScript
  (bind _garagedoor (Variables|Default|GetGarageDoor))
  (if (Variables|Default|GetDoorOpen)
    (Transformation|SetRelativeLocation _garagedoor (Math|Vector|MakeVector 3.3 -18.5 2.3e+02) false true)
    (else
      (Transformation|SetRelativeLocation _garagedoor (Math|Vector|MakeVector 3.3 -18.5 31.0) false true))))

(fn EventTryUse
  (params (Pawn :type INS%20Soldier%20Object%20Reference) (HitResult :type Hit%20Result%20Structure%20%28by%20ref%29))
  (Networking|SwitchHasAuthority
    (:Authority
      _)
    (:Remote
      _))
  (CallFunction|Switch)
  (return "HandledServer"))

(fn SwitchServer)

(fn OnRepDoorOpen)

(fn OnRepCanOpen?)